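; BP_Item is an item actor with a name, an elemental type and type-dependent damage, printing debug text on BeginPlay.
; An empty name gets a pick from four hardcoded names, though the random index's upper bound is the negated array length.
; GetDamage zeroes damage when the item's element is two enum steps from the victim's, using modulo four.
; BeginPlay tests this against a Fire victim; other damage logic is unconnected.
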(event `self.ReceiveBeginPlay`
  (`self.Constructor Function`)
  (`KismetSystemLibrary.PrintString` (`KismetStringLibrary.Concat_StrStr` "Hello my name is" (`self.Name`)))
  (bind _damage (`self.Get Damage` "NewEnumerator0"))
  (`KismetSystemLibrary.PrintString` (`KismetStringLibrary.Concat_StrStr` "Our Elemental type is " (`|GetEnumeratorNameAsString` (`self.ElementalType`)) "water the victum is fire that damage is =" (`KismetStringLibrary.Conv_IntToString` _damage)) true true (struct :`R` 1.0 :`G` 0.184 :`B` 0.184 :`A` 1.0)))

(fn `Constructor Function`
  (bind _array (`|MakeArray` "Larry" "Lana" "Perry" "Penny"))
  (if (`KismetStringLibrary.EqualEqual_StrStr` (`self.Name`))
    (`KismetArrayLibrary.Array_Shuffle` _array)
    (set `self.Name` (`KismetTextLibrary.Conv_TextToString` (`|GetArrayItem` _array (`KismetMathLibrary.RandomIntegerInRange` 0 (- 0 (`KismetArrayLibrary.Array_Length` _array))))))))

(fn `Get Damage`
  (params (` VictumElementalType` :type "/Game/BluePrints/ElementalType Enum" :default "NewEnumerator1"))
  (returns (Damage :type Integer))
  (locals (`Returned Damaged` :type Integer :default 0))
  (set `local.Returned Damaged` (`self.Damage`))
  (if (== (mod (+ ` VictumElementalType` 2) 4) (`KismetMathLibrary.Conv_ByteToInt` (`self.ElementalType`)))
    (set `local.Returned Damaged` (* (`self.Damage`) 0)))
  (return (`local.Returned Damaged`)))

(fn `UserConstructionScript`)